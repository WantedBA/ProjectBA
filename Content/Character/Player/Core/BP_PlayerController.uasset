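; Player controller that creates the main HUD and binds debug-style keys to exercise its widgets.
; On BeginPlay it pushes WBP_MainHUD through the UI subsystem and caches the reference.
; Keys 1 and 2 feed hardcoded counts and cooldowns to the HP and stamina quickslots, and key 5 shows a test boss status bar, with no gameplay data behind them.
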(event EventBeginPlay
  ;[0.15 0.15 0.15 0.5] HUD
  (bind _returnvalue (Class|SubSystemUI|PushUIbyClass (Subsystems|GetSubSystemUI) "/Game/UI/HUD/WBP_MainHUD.WBP_MainHUD_C"))
  (bind _aswbp_main_hud (Utilities|Casting|CastToWBP_MainHUD _returnvalue))
  (Variables|Default|SetMainHUDRef _aswbp_main_hud))

(event EventTick
  (params (DeltaSeconds :type Float%20%28single-precision%29)))

(event Input|KeyboardEvents|5
  (params (Key :type Key%20Structure :default "None"))
  ;[0.15 0.15 0.15 0.5] Boss HP 테스트
  (:Pressed
    (Class|MainHUD|UpdateBossStatus (Variables|Default|GetMainHUDRef) "테스트 보스" 1e+02 1e+02)))

(event Input|KeyboardEvents|1
  (params (Key :type Key%20Structure :default "None"))
  (bind _mainhudref (Variables|Default|GetMainHUDRef))
  (bind _hpslot (Variables|/Script/BAProject.MainHUD|GetHPSlot _mainhudref))
  ;[0.15 0.15 0.15 0.5] HP 퀵슬롯
  (:Pressed
    (Class|QuickSlotBase|UpdateCount _hpslot 10)
    (Class|QuickSlotBase|StartCooldown _hpslot 5.0)))

(event Input|KeyboardEvents|2
  (params (Key :type Key%20Structure :default "None"))
  (bind _mainhudref (Variables|Default|GetMainHUDRef))
  (bind _staminaslot (Variables|/Script/BAProject.MainHUD|GetStaminaSlot _mainhudref))
  ;[0.15 0.15 0.15 0.5] Stamina 퀵슬롯
  (:Pressed
    (Class|QuickSlotBase|UpdateCount _staminaslot 10)
    (Class|QuickSlotBase|StartCooldown _staminaslot 5.0)))

(fn ConstructionScript)